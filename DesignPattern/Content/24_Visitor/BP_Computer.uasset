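; BP_Computer is the composite element in a Visitor design pattern example, representing a computer built from parts.
; On BeginPlay it spawns mouse, keyboard and monitor actors and stores them in ComputerParts.
; Accept loops over those parts, passing the visitor to each part's Accept, and calls Visit on itself inside the loop, so the computer is visited once per part.
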(event EventBeginPlay
  (bind _returnvalue (Game|SpawnActorfromClass "/Game/24_Visitor/BP_Mouse.BP_Mouse_C" (Math|Transform|MakeTransform "0, 0, 0" "0, 0, 0" "1,1,1") "Undefined" 0 0))
  (Utilities|Array|Add (Variables|Default|GetComputerParts) _returnvalue)
  (bind _returnvalue_2 (Game|SpawnActorfromClass "/Game/24_Visitor/BP_Keyboard.BP_Keyboard_C" (Math|Transform|MakeTransform "0, 0, 0" "0, 0, 0" "1,1,1") "Undefined" 0 0))
  (Utilities|Array|Add (Variables|Default|GetComputerParts) _returnvalue_2)
  (bind _returnvalue_3 (Game|SpawnActorfromClass "/Game/24_Visitor/BP_Monitor.BP_Monitor_C" (Math|Transform|MakeTransform "0, 0, 0" "0, 0, 0" "1,1,1") "Undefined" 0 0))
  (Utilities|Array|Add (Variables|Default|GetComputerParts) _returnvalue_3))

(fn ConstructionScript
  (|CallParentFunction))

(fn Accept
  (params (ComputerPartVisitor :type BP%20Computer%20Part%20Visitor%20Object%20Reference))
  (for _array_element (Variables|Default|GetComputerParts)
    (CallFunction|Accept _array_element ComputerPartVisitor)
    (Default|Visit ComputerPartVisitor self)))