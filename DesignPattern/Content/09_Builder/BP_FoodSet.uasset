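; BP_FoodSet is a food set that holds a collection of items, apparently the product in a Builder pattern example.
; AddItem appends to the Items array, which the other functions loop over.
; GetCost adds each item's Price to Cost and returns it, with no reset shown in the function.
; ShowItem prints each item's Name.
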(fn ConstructionScript)

(fn AddItem
  (params (Item :type BP%20Item%20Object%20Reference))
  (Utilities|Array|Add (Variables|Default|GetItems) Item))

(fn GetCost
  (for _array_element (Variables|Default|GetItems)
    (bind _price (Default|Price _array_element))
    (LocalVariables|SetCost (+ (LocalVariables|GetCost) _price)))
  (return (LocalVariables|GetCost)))

(fn ShowItem
  (for _array_element (Variables|Default|GetItems)
    (bind _name (Default|Name _array_element))
    (Development|PrintString _name)))