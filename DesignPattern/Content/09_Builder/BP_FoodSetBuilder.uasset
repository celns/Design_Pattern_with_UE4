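; BP_FoodSetBuilder is a Builder pattern Blueprint that assembles preset vegetarian and non-vegetarian food sets.
; Each build function spawns a BP_FoodSet actor, spawns a burger and a drink, adds both through AddItem, and returns the set.
; The veg set pairs a veg burger with Coka, and the non-veg set pairs a chicken burger with Pepsi.
; The event graph and construction script contain no logic.
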(event EventBeginPlay)

(event Collision|EventActorBeginOverlap
  (params (OtherActor :type Actor%20Object%20Reference)))

(event EventTick
  (params (DeltaSeconds :type Float%20%28single-precision%29)))

(fn ConstructionScript)

(fn BuildVegFoodSet
  (bind _returnvalue (Game|SpawnActorfromClass "/Game/09_Builder/BP_FoodSet.BP_FoodSet_C" (Math|Transform|MakeTransform "0, 0, 0" "0, 0, 0" "1,1,1") "Undefined" 0 0))
  (Utilities|FlowControl|Sequence
    (:then_0
      (bind _returnvalue_2 (Game|SpawnActorfromClass "/Game/09_Builder/Item/Burger/BP_VegBurger.BP_VegBurger_C" (Math|Transform|MakeTransform "0, 0, 0" "0, 0, 0" "1,1,1") "Undefined" 0 0))
      (Default|AddItem _returnvalue _returnvalue_2))
    (:then_1
      (bind _returnvalue_3 (Game|SpawnActorfromClass "/Game/09_Builder/Item/Colddrink/BP_Coka.BP_Coka_C" (Math|Transform|MakeTransform "0, 0, 0" "0, 0, 0" "1,1,1") "Undefined" 0 0))
      (Default|AddItem _returnvalue _returnvalue_3))
    (:then_2
      (return _returnvalue))))

(fn BuildNonVegFoodSet
  (bind _returnvalue (Game|SpawnActorfromClass "/Game/09_Builder/BP_FoodSet.BP_FoodSet_C" (Math|Transform|MakeTransform "0, 0, 0" "0, 0, 0" "1,1,1") "Undefined" 0 0))
  (Utilities|FlowControl|Sequence
    (:then_0
      (bind _returnvalue_2 (Game|SpawnActorfromClass "/Game/09_Builder/Item/Burger/BP_ChickenBurger.BP_ChickenBurger_C" (Math|Transform|MakeTransform "0, 0, 0" "0, 0, 0" "1,1,1") "Undefined" 0 0))
      (Default|AddItem _returnvalue _returnvalue_2))
    (:then_1
      (bind _returnvalue_3 (Game|SpawnActorfromClass "/Game/09_Builder/Item/Colddrink/BP_Pepsi.BP_Pepsi_C" (Math|Transform|MakeTransform "0, 0, 0" "0, 0, 0" "1,1,1") "Undefined" 0 0))
      (Default|AddItem _returnvalue _returnvalue_3))
    (:then_2
      (return _returnvalue))))