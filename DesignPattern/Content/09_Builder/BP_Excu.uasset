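; BP_Excu is a demo actor that exercises a Builder pattern for food sets.
; On BeginPlay it spawns a BP_FoodSetBuilder and asks it for a vegetarian set, then a non-vegetarian set.
; For each built set it prints the total cost and calls ShowItem to display the contents.
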(event EventBeginPlay
  (bind _returnvalue (Game|SpawnActorfromClass "/Game/09_Builder/BP_FoodSetBuilder.BP_FoodSetBuilder_C" (Math|Transform|MakeTransform "0, 0, 0" "0, 0, 0" "1,1,1") "Undefined" 0 0))
  (Utilities|FlowControl|Sequence
    (:then_0
      (bind _foodset (Default|BuildVegFoodSet _returnvalue))
      (Utilities|FlowControl|Sequence
        (:then_0
          (bind _totalcost (Default|GetCost _foodset))
          (Development|PrintString (Utilities|String|ToString(Float) _totalcost)))
        (:then_1
          (Default|ShowItem _foodset))))
    (:then_1
      (bind _foodset_2 (Default|BuildNonVegFoodSet _returnvalue))
      (Utilities|FlowControl|Sequence
        (:then_0
          (bind _totalcost_2 (Default|GetCost _foodset_2))
          (Development|PrintString (Utilities|String|ToString(Float) _totalcost_2)))
        (:then_1
          (Default|ShowItem _foodset_2))))))

(fn ConstructionScript)