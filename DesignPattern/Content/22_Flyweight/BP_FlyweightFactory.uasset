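; Flyweight factory from a Flyweight design pattern example, which creates and hands out shared BP_ConcreteFlyweight actors by key.
; On BeginPlay it spawns three flyweight actors and stores them in the Flyweights map under fixed string keys.
; GetFlywieght looks up a key and returns the existing actor when found; it does not create flyweights for missing keys.
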(event EventBeginPlay
  (Utilities|FlowControl|Sequence
    (:then_0
      (bind _returnvalue (Game|SpawnActorfromClass "/Game/22_Flyweight/BP_ConcreteFlyweight.BP_ConcreteFlyweight_C" (Math|Transform|MakeTransform "0, 0, 0" "0, 0, 0" "1,1,1") "Undefined" 0 0))
      (Utilities|Map|Add (Variables|Default|GetFlyweights) "X" _returnvalue))
    (:then_1
      (bind _returnvalue_2 (Game|SpawnActorfromClass "/Game/22_Flyweight/BP_ConcreteFlyweight.BP_ConcreteFlyweight_C" (Math|Transform|MakeTransform "1.000000,1.000000,1.000000" "0, 0, 0" "1,1,1") "Undefined" 0 0))
      (Utilities|Map|Add (Variables|Default|GetFlyweights) "Y" _returnvalue_2))
    (:then_2
      (bind _returnvalue_3 (Game|SpawnActorfromClass "/Game/22_Flyweight/BP_ConcreteFlyweight.BP_ConcreteFlyweight_C" (Math|Transform|MakeTransform "2.000000,2.000000,2.000000" "0, 0, 0" "1,1,1") "Undefined" 0 0))
      (Utilities|Map|Add (Variables|Default|GetFlyweights) "Z" _returnvalue_3))))

(fn ConstructionScript)

(fn GetFlywieght
  (params (Key :type String))
  (bind _flyweights (Variables|Default|GetFlyweights))
  (bind (_value _returnvalue) (Utilities|Map|Find _flyweights Key))
  (if _returnvalue
    (return _value)))