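; BP_Excu is the client that exercises a Flyweight design pattern example on BeginPlay.
; It spawns a BP_FlyweightFactory, requests flyweights by string key and calls Operation on each with a decremented Extrin value as extrinsic state.
; It then spawns a BP_UnsharedConcreteFlyweight directly, bypassing the factory, and calls Operation on it the same way.
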(event EventBeginPlay
  (Utilities|FlowControl|Sequence
    (:then_0
      (bind _returnvalue (Game|SpawnActorfromClass "/Game/22_Flyweight/BP_FlyweightFactory.BP_FlyweightFactory_C" (Math|Transform|MakeTransform "0, 0, 0" "0, 0, 0" "1,1,1") "Undefined" 0 0))
      (Utilities|FlowControl|Sequence
        (:then_0
          (bind _flyweight (Default|GetFlywieght _returnvalue "X"))
          (bind _result (Math|Integer|DecrementInt (Variables|Default|Getextrin))
            (:%20%20
              (Default|Operation _flyweight _result))))
        (:then_1
          (bind _flyweight_2 (Default|GetFlywieght _returnvalue "Y"))
          (bind _result_2 (Math|Integer|DecrementInt (Variables|Default|Getextrin))
            (:%20%20
              (Default|Operation _flyweight_2 _result_2))))
        (:then_2
          (bind _flyweight_3 (Default|GetFlywieght _returnvalue "Z"))
          (bind _result_3 (Math|Integer|DecrementInt (Variables|Default|Getextrin))
            (:%20%20
              (Default|Operation _flyweight_3 _result_3))))))
    (:then_1
      (bind _returnvalue_2 (Game|SpawnActorfromClass "/Game/22_Flyweight/BP_UnsharedConcreteFlyweight.BP_UnsharedConcreteFlyweight_C" (Math|Transform|MakeTransform "0, 0, 0" "0, 0, 0" "1,1,1") "Undefined" 0 0))
      (bind _result_4 (Math|Integer|DecrementInt (Variables|Default|Getextrin))
        (:%20%20
          (Default|Operation _returnvalue_2 _result_4))))))

(fn ConstructionScript)