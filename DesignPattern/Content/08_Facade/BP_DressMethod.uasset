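; BP_DressMethod is the facade in a Facade pattern example, wrapping three skin actors behind simple dress functions.
; On BeginPlay it spawns and stores BP_SkinAsh, BP_SkinBet and BP_SkinCat.
; DressAll prints its name and triggers the VFX function on all three skins, while DressTwo does the same for Bet and Ash only.
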(event EventBeginPlay
  (Utilities|FlowControl|Sequence
    (:then_0
      (bind _returnvalue (Game|SpawnActorfromClass "/Game/08_Facade/BP_SkinAsh.BP_SkinAsh_C" (Math|Transform|MakeTransform "0, 0, 0" "0, 0, 0" "1,1,1") "Undefined" 0 0))
      (Variables|Default|SetAsh _returnvalue))
    (:then_1
      (bind _returnvalue_2 (Game|SpawnActorfromClass "/Game/08_Facade/BP_SkinBet.BP_SkinBet_C" (Math|Transform|MakeTransform "0, 0, 0" "0, 0, 0" "1,1,1") "Undefined" 0 0))
      (Variables|Default|SetBet _returnvalue_2))
    (:then_2
      (bind _returnvalue_3 (Game|SpawnActorfromClass "/Game/08_Facade/BP_SkinCat.BP_SkinCat_C" (Math|Transform|MakeTransform "0, 0, 0" "0, 0, 0" "1,1,1") "Undefined" 0 0))
      (Variables|Default|SetCat _returnvalue_3))))

(fn ConstructionScript)

(fn DressAll
  (Utilities|FlowControl|Sequence
    (:then_0
      (Development|PrintString "DressAll:"))
    (:then_1
      (Default|VFXAsh (Variables|Default|GetAsh)))
    (:then_2
      (Default|VFXBet (Variables|Default|GetBet)))
    (:then_3
      (Default|VFXCat (Variables|Default|GetCat)))))

(fn DressTwo
  (Utilities|FlowControl|Sequence
    (:then_0
      (Development|PrintString "DressTwo"))
    (:then_1
      (Default|VFXBet (Variables|Default|GetBet)))
    (:then_2
      (Default|VFXAsh (Variables|Default|GetAsh)))))