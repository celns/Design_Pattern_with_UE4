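; BP_IndustryCity is the composite node in a Composite pattern example, representing a city that holds child cities.
; AddDuty and RmoveDuty add and remove entries in the ChildrenCity array.
; DisplayDuty and LineOfDuty forward recursively to every child, with DisplayDuty increasing the depth at each level, and neither does work of its own.
; The event graph holds only disabled default events.
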(event EventBeginPlay
  (|CallParentFunction) ; 此节点被禁用，将不会被调用。\n从引脚连出引线来编译功能。
)

(event Collision|EventActorBeginOverlap
  (params (OtherActor :type Actor%20Object%20Reference))
  (|CallParentFunction OtherActor) ; 此节点被禁用，将不会被调用。\n从引脚连出引线来编译功能。
)

(event EventTick
  (params (DeltaSeconds :type Float%20%28single-precision%29))
  (|CallParentFunction DeltaSeconds) ; 此节点被禁用，将不会被调用。\n从引脚连出引线来编译功能。
)

(fn ConstructionScript
  (|CallParentFunction))

(fn AddDuty
  (params (City :type BP%20City%20Object%20Reference))
  (Utilities|Array|Add (Variables|Default|GetChildrenCity) City))

(fn RmoveDuty
  (params (City :type BP%20City%20Object%20Reference))
  (Utilities|Array|RemoveItem (Variables|Default|GetChildrenCity) City))

(fn DisplayDuty
  (params (Depth :type Integer))
  (for _array_element (Variables|Default|GetChildrenCity)
    (CallFunction|DisplayDuty _array_element (+ Depth 2))))

(fn LineOfDuty
  (for _array_element (Variables|Default|GetChildrenCity)
    (CallFunction|LineOfDuty _array_element)))