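; BP_Excu is a driver actor for a Composite pattern example, judging by its folder, that builds and exercises an industry city hierarchy at BeginPlay.
; It spawns a BP_IndustryCity, then spawns Ficility, Finance and PublicService actors and registers each with the city through AddDuty.
; It then calls DisplayDuty and LineOfDuty on the city alone.
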(event EventBeginPlay
  (Utilities|FlowControl|Sequence
    (:then_0
      (bind _returnvalue (Game|SpawnActorfromClass "/Game/15_Composite/BP_IndustryCity.BP_IndustryCity_C" (Math|Transform|MakeTransform "0, 0, 0" "0, 0, 0" "1,1,1") "Undefined" 0 "IndustryCity" 0))
      (Utilities|FlowControl|Sequence
        (:then_0
          (bind _returnvalue_2 (Game|SpawnActorfromClass "/Game/15_Composite/BP_Ficility.BP_Ficility_C" (Math|Transform|MakeTransform "0, 0, 0" "0, 0, 0" "1,1,1") "Undefined" 0 "Ficility" 0))
          (Default|AddDuty _returnvalue _returnvalue_2))
        (:then_1
          (bind _returnvalue_3 (Game|SpawnActorfromClass "/Game/15_Composite/BP_Finance.BP_Finance_C" (Math|Transform|MakeTransform "0, 0, 0" "0, 0, 0" "1,1,1") "Undefined" 0 "Finance" 0))
          (Default|AddDuty _returnvalue _returnvalue_3))
        (:then_2
          (bind _returnvalue_4 (Game|SpawnActorfromClass "/Game/15_Composite/BP_PublicService.BP_PublicService_C" (Math|Transform|MakeTransform "0, 0, 0" "0, 0, 0" "1,1,1") "Undefined" 0 "PublicService" 0))
          (Default|AddDuty _returnvalue _returnvalue_4))))
    (:then_1
      (Default|DisplayDuty _returnvalue 2)
      (Default|LineOfDuty _returnvalue))))

(fn ConstructionScript)