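; BP_Excu is a demo driver for an Iterator pattern over treasure items.
; On BeginPlay it spawns a BP_TresureRepo and fills its Items array with three BP_TresureItem actors placed at different locations.
; It then spawns a BP_TresureIterator bound to that repo and walks it with First and Next.
; Each item's location and the final HasNext result are printed to verify the traversal.
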(event EventBeginPlay
  (Utilities|FlowControl|Sequence
    (:then_0
      (bind _returnvalue (Game|SpawnActorfromClass "/Game/16_Iterator/BP_TresureRepo.BP_TresureRepo_C" (Math|Transform|MakeTransform "0, 0, 0" "0, 0, 0" "1,1,1") "Undefined" 0 0))
      (Utilities|FlowControl|Sequence
        (:then_0
          (bind _returnvalue_2 (Game|SpawnActorfromClass "/Game/16_Iterator/BP_TresureItem.BP_TresureItem_C" (Math|Transform|MakeTransform "10.000000,10.000000,10.000000" "0, 0, 0" "1,1,1") "Undefined" 0 0))
          (Utilities|Array|Add (Variables|/Game/16_Iterator/BP_TresureRepo.BP_TresureRepo_C|GetItems _returnvalue) _returnvalue_2))
        (:then_1
          (bind _returnvalue_3 (Game|SpawnActorfromClass "/Game/16_Iterator/BP_TresureItem.BP_TresureItem_C" (Math|Transform|MakeTransform "20.000000,20.000000,20.000000" "0, 0, 0" "1,1,1") "Undefined" 0 0))
          (Utilities|Array|Add (Variables|/Game/16_Iterator/BP_TresureRepo.BP_TresureRepo_C|GetItems _returnvalue) _returnvalue_3))
        (:then_2
          (bind _returnvalue_4 (Game|SpawnActorfromClass "/Game/16_Iterator/BP_TresureItem.BP_TresureItem_C" (Math|Transform|MakeTransform "30.000000,30.000000,30.000000" "0, 0, 0" "1,1,1") "Undefined" 0 0))
          (Utilities|Array|Add (Variables|/Game/16_Iterator/BP_TresureRepo.BP_TresureRepo_C|GetItems _returnvalue) _returnvalue_4))))
    (:then_1
      (bind _returnvalue_5 (Game|SpawnActorfromClass "/Game/16_Iterator/BP_TresureIterator.BP_TresureIterator_C" (Math|Transform|MakeTransform "0, 0, 0" "0, 0, 0" "1,1,1") "Undefined" 0 _returnvalue 0))
      (Utilities|FlowControl|Sequence
        (:then_0
          (bind _actor (Default|First _returnvalue_5))
          (Development|PrintString (Utilities|String|ToString(Vector) (.location (Transformation|GetActorTransform _actor)))))
        (:then_1
          (bind _next (Default|Next _returnvalue_5))
          (Development|PrintString (Utilities|String|ToString(Vector) (.location (Transformation|GetActorTransform _next)))))
        (:then_2
          (bind _next_2 (Default|Next _returnvalue_5))
          (Development|PrintString (Utilities|String|ToString(Vector) (.location (Transformation|GetActorTransform _next_2)))))
        (:then_3
          (bind _hasnext (Default|HasNext _returnvalue_5))
          (Development|PrintString (Utilities|String|Append "HasNext:" (Utilities|String|ToString(Boolean) _hasnext))))))))

(fn ConstructionScript)