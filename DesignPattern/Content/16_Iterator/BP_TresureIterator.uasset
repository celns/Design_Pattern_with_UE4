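; BP_TresureIterator is an Iterator pattern Blueprint that walks the items held by a TresureRepo in order.
; First returns item zero without resetting Index, and CurrentItem returns the item at Index.
; HasNext checks the following index against the repo's count, and Next uses it to guard advancing Index and returning that item.
; The event graph has no active logic.
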(event EventBeginPlay)

(event Collision|EventActorBeginOverlap
  (params (OtherActor :type Actor%20Object%20Reference))
  (|CallParentFunction OtherActor) ; 此节点被禁用，将不会被调用。\n从引脚连出引线来编译功能。
)

(event EventTick
  (params (DeltaSeconds :type Float%20%28single-precision%29))
  (|CallParentFunction DeltaSeconds) ; 此节点被禁用，将不会被调用。\n从引脚连出引线来编译功能。
)

(fn ConstructionScript
  (|CallParentFunction))

(fn HasNext
  (bind _count (Default|GetCount (Variables|Default|GetTresureRepo)))
  (return (< (+ (Variables|Default|GetIndex) 1) _count)))

(fn First
  (return (Utilities|Array|Get(acopy) (Variables|/Game/16_Iterator/BP_TresureRepo.BP_TresureRepo_C|GetItems (Variables|Default|GetTresureRepo)))))

(fn Next
  (bind _hasnext (CallFunction|HasNext))
  (if _hasnext
    (Math|Integer|IncrementInt (Variables|Default|GetIndex)
      (:%20%20
        (return (Utilities|Array|Get(acopy) (Variables|/Game/16_Iterator/BP_TresureRepo.BP_TresureRepo_C|GetItems (Variables|Default|GetTresureRepo)) (Variables|Default|GetIndex)))))))

(fn CurrentItem
  (return (Utilities|Array|Get(acopy) (Variables|/Game/16_Iterator/BP_TresureRepo.BP_TresureRepo_C|GetItems (Variables|Default|GetTresureRepo)) (Variables|Default|GetIndex))))