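; BP_CommandMove is a move command actor that follows the Command pattern, wrapping an action request to a receiver object.
; Its Excute function calls Action on the Receiver, then prints "Move" as feedback.
; The event graph holds only disabled default events, so the command does nothing until Excute is called.
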(event EventBeginPlay
  (|CallParentFunction) ; 此节点被禁用，将不会被调用。\n从引脚连出引线来编译功能。
)

(event Collision|EventActorBeginOverlap
  (params (OtherActor :type Actor%20Object%20Reference))
  (|CallParentFunction OtherActor) ; 此节点被禁用，将不会被调用。\n从引脚连出引线来编译功能。
)

(event EventTick
  (params (DeltaSeconds :type Float%20%28single-precision%29))
  (|CallParentFunction DeltaSeconds) ; 此节点被禁用，将不会被调用。\n从引脚连出引线来编译功能。
)

(fn ConstructionScript
  (|CallParentFunction))

(fn Excute
  (Default|Action (Variables|Default|GetReceiver))
  (Development|PrintString "Move"))