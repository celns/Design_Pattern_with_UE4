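; BP_PotionFactory is a concrete factory in an Abstract Factory example that creates potion actors.
; GetPotion switches on the requested potion type, then spawns and returns a heal, toxin or mana potion actor.
; GetSize only forwards to the parent implementation with a fixed enum value, ignoring its Size input.
; The event graph holds only disabled default events, so the factory acts only when called.
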(event EventBeginPlay
  (|CallParentFunction) ; 此节点被禁用，将不会被调用。\n从引脚连出引线来编译功能。
)

(event Collision|EventActorBeginOverlap
  (params (OtherActor :type Actor%20Object%20Reference))
  (|CallParentFunction OtherActor) ; 此节点被禁用，将不会被调用。\n从引脚连出引线来编译功能。
)

(event EventTick
  (params (DeltaSeconds :type Float%20%28single-precision%29))
  (|CallParentFunction DeltaSeconds) ; 此节点被禁用，将不会被调用。\n从引脚连出引线来编译功能。
)

(fn ConstructionScript
  (|CallParentFunction))

(fn GetPotion
  (params (PotionType :type PotionType%20Enum :default "NewEnumerator0"))
  (switch Utilities|FlowControl|Switch|SwitchonPotionType PotionType
    (:NewEnumerator0
      (bind _returnvalue (Game|SpawnActorfromClass "/Game/11_AbstractFactory/Potion/BP_HealPotion.BP_HealPotion_C" (Math|Transform|MakeTransform "0, 0, 0" "0, 0, 0" "1,1,1") "Undefined" 0 0))
      (return _returnvalue))
    (:NewEnumerator1
      (bind _returnvalue_2 (Game|SpawnActorfromClass "/Game/11_AbstractFactory/Potion/BP_ToxinPotion.BP_ToxinPotion_C" (Math|Transform|MakeTransform "0, 0, 0" "0, 0, 0" "1,1,1") "Undefined" 0 0))
      (return _returnvalue_2))
    (:NewEnumerator2
      (bind _returnvalue_3 (Game|SpawnActorfromClass "/Game/11_AbstractFactory/Potion/BP_ManaPotion.BP_ManaPotion_C" (Math|Transform|MakeTransform "0, 0, 0" "0, 0, 0" "1,1,1") "Undefined" 0 0))
      (return _returnvalue_3))))

(fn GetSize
  (params (Size :type PotionSizeType%20Enum :default "NewEnumerator0"))
  (bind _potionsize (|CallParentFunction "NewEnumerator0"))
  (return _potionsize))