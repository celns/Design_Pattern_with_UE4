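; BP_Excu is a demo driver for the Abstract Factory pattern, exercising potion and size factories when play begins.
; It spawns a BP_FactoryProducer, which returns a concrete factory for a given string key.
; The Potion factory supplies two potion types whose Buff is called, then the Size factory supplies a size object whose Size is called.
; Products are chosen by enum, so the caller only invokes GetPotion, GetSize and their methods.
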(event EventBeginPlay
  (bind _returnvalue (Game|SpawnActorfromClass "/Game/11_AbstractFactory/BP_FactoryProducer.BP_FactoryProducer_C" (Math|Transform|MakeTransform "0, 0, 0" "0, 0, 0" "1,1,1") "Undefined" 0 0))
  (Utilities|FlowControl|Sequence
    (:then_0
      (bind _factory (Default|GetFactory _returnvalue "Potion"))
      (Utilities|FlowControl|Sequence
        (:then_0
          (bind _potion (Default|GetPotion _factory "NewEnumerator0"))
          (Default|Buff _potion))
        (:then_1
          (bind _potion_2 (Default|GetPotion _factory "NewEnumerator2"))
          (Default|Buff _potion_2))))
    (:then_1
      (bind _factory_2 (Default|GetFactory _returnvalue "Size"))
      (bind _potionsize (Default|GetSize _factory_2 "NewEnumerator0"))
      (Default|Size _potionsize))))

(fn ConstructionScript)