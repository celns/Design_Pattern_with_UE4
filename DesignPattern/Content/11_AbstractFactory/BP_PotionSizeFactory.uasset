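; BP_PotionSizeFactory is an actor that serves as the potion size factory in an Abstract Factory example.
; GetSize switches on the requested size and spawns the matching BP_SmallSize, BP_LargeSize or BP_FullSize actor, returning the new instance.
; The event graph holds only disabled default events, so all of its own logic lives in that one function.
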(event EventBeginPlay
  (|CallParentFunction) ; 此节点被禁用，将不会被调用。\n从引脚连出引线来编译功能。
)

(event Collision|EventActorBeginOverlap
  (params (OtherActor :type Actor%20Object%20Reference))
  (|CallParentFunction OtherActor) ; 此节点被禁用，将不会被调用。\n从引脚连出引线来编译功能。
)

(event EventTick
  (params (DeltaSeconds :type Float%20%28single-precision%29))
  (|CallParentFunction DeltaSeconds) ; 此节点被禁用，将不会被调用。\n从引脚连出引线来编译功能。
)

(fn ConstructionScript
  (|CallParentFunction))

(fn GetSize
  (params (Size :type PotionSizeType%20Enum :default "NewEnumerator0"))
  (switch Utilities|FlowControl|Switch|SwitchonPotionSizeType Size
    (:NewEnumerator0
      (bind _returnvalue (Game|SpawnActorfromClass "/Game/11_AbstractFactory/PotionSize/BP_SmallSize.BP_SmallSize_C" (Math|Transform|MakeTransform "0, 0, 0" "0, 0, 0" "1,1,1") "Undefined" 0 0))
      (return _returnvalue))
    (:NewEnumerator1
      (bind _returnvalue_2 (Game|SpawnActorfromClass "/Game/11_AbstractFactory/PotionSize/BP_LargeSize.BP_LargeSize_C" (Math|Transform|MakeTransform "0, 0, 0" "0, 0, 0" "1,1,1") "Undefined" 0 0))
      (return _returnvalue_2))
    (:NewEnumerator2
      (bind _returnvalue_3 (Game|SpawnActorfromClass "/Game/11_AbstractFactory/PotionSize/BP_FullSize.BP_FullSize_C" (Math|Transform|MakeTransform "0, 0, 0" "0, 0, 0" "1,1,1") "Undefined" 0 0))
      (return _returnvalue_3))))