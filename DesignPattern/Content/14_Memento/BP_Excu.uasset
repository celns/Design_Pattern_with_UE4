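; BP_Excu is a demo driver for the Memento design pattern, running entirely on BeginPlay.
; It spawns an Originator, sets its state to "On" and shows it.
; It then spawns a CareTaker, stores a memento created by the Originator in it and switches the state to "Off".
; Finally, it hands the stored memento back to the Originator, showing the state after each change.
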(event EventBeginPlay
  (Utilities|FlowControl|Sequence
    (:then_0
      (bind _returnvalue (Game|SpawnActorfromClass "/Game/14_Memento/BP_Originator.BP_Originator_C" (Math|Transform|MakeTransform "0, 0, 0" "0, 0, 0" "1,1,1") "Undefined" 0 0))
      (Variables|/Game/14_Memento/BP_Originator.BP_Originator_C|SetState _returnvalue "On")
      (Default|ShowState _returnvalue))
    (:then_1
      (bind _returnvalue_2 (Game|SpawnActorfromClass "/Game/14_Memento/BP_CareTaker.BP_CareTaker_C" (Math|Transform|MakeTransform "0, 0, 0" "0, 0, 0" "1,1,1") "Undefined" 0 0))
      (bind _memento (Default|CreateMememto _returnvalue))
      (Variables|/Game/14_Memento/BP_CareTaker.BP_CareTaker_C|SetMemento _returnvalue_2 _memento)
      (Variables|/Game/14_Memento/BP_Originator.BP_Originator_C|SetState _returnvalue "Off")
      (Default|ShowState _returnvalue)
      (Default|SetMemento _returnvalue (Variables|/Game/14_Memento/BP_CareTaker.BP_CareTaker_C|GetMemento _returnvalue_2))
      (Default|ShowState _returnvalue))))

(fn ConstructionScript)