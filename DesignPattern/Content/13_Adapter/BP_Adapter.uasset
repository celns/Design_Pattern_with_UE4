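; BP_Adapter is an actor that demonstrates the Adapter design pattern, exposing a Request function in place of the adaptee's own interface.
; On BeginPlay it spawns a BP_Adaptee actor and stores the reference.
; Request forwards to SpecificRequest on that stored instance, so the adapter wraps the adaptee by composition.
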(event EventBeginPlay
  (bind _returnvalue (Game|SpawnActorfromClass "/Game/13_Adapter/BP_Adaptee.BP_Adaptee_C" (Math|Transform|MakeTransform "0, 0, 0" "0, 0, 0" "1,1,1") "Undefined" 0 0))
  (Variables|Default|SetAdaptee _returnvalue))

(event Collision|EventActorBeginOverlap
  (params (OtherActor :type Actor%20Object%20Reference))
  (|CallParentFunction OtherActor) ; 此节点被禁用，将不会被调用。\n从引脚连出引线来编译功能。
)

(event EventTick
  (params (DeltaSeconds :type Float%20%28single-precision%29))
  (|CallParentFunction DeltaSeconds) ; 此节点被禁用，将不会被调用。\n从引脚连出引线来编译功能。
)

(fn ConstructionScript
  (|CallParentFunction))

(fn Request
  (Default|SpecificRequest (Variables|Default|GetAdaptee)))