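; BP_Excu is a demo driver actor for the Bridge design pattern, running a refined abstraction with swappable magic implementors.
; On BeginPlay it spawns one BP_RefinedAbstraction, then uses a Sequence to spawn fire, ice and toxin magic actors in turn.
; Each is passed to SetImplementor before Operation is called, so the same abstraction runs with each implementation.
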(event EventBeginPlay
  (bind _returnvalue (Game|SpawnActorfromClass "/Game/18_Bridge/BP_RefinedAbstraction.BP_RefinedAbstraction_C" (Math|Transform|MakeTransform "0, 0, 0" "0, 0, 0" "1,1,1") "Undefined" 0 0))
  (Utilities|FlowControl|Sequence
    (:then_0
      (bind _returnvalue_2 (Game|SpawnActorfromClass "/Game/18_Bridge/BP_FireMagic.BP_FireMagic_C" (Math|Transform|MakeTransform "0, 0, 0" "0, 0, 0" "1,1,1") "Undefined" 0 0))
      (Default|SetImplementor _returnvalue _returnvalue_2)
      (Default|Operation _returnvalue))
    (:then_1
      (bind _returnvalue_3 (Game|SpawnActorfromClass "/Game/18_Bridge/BP_IceMagic.BP_IceMagic_C" (Math|Transform|MakeTransform "0, 0, 0" "0, 0, 0" "1,1,1") "Undefined" 0 0))
      (Default|SetImplementor _returnvalue _returnvalue_3)
      (Default|Operation _returnvalue))
    (:then_2
      (bind _returnvalue_4 (Game|SpawnActorfromClass "/Game/18_Bridge/BP_ToxinMagic.BP_ToxinMagic_C" (Math|Transform|MakeTransform "0, 0, 0" "0, 0, 0" "1,1,1") "Undefined" 0 0))
      (Default|SetImplementor _returnvalue _returnvalue_4)
      (Default|Operation _returnvalue))))

(event Collision|EventActorBeginOverlap
  (params (OtherActor :type Actor%20Object%20Reference)))

(event EventTick
  (params (DeltaSeconds :type Float%20%28single-precision%29)))

(fn ConstructionScript)