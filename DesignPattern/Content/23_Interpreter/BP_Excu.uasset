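; BP_Excu is a demo driver actor for the Interpreter design pattern, run on BeginPlay.
; A sequence spawns two terminal expression actors and one non-terminal expression actor, adding each to ExpressionList.
; It then spawns a BP_InterpreterContext and calls Interpret on every listed expression in order, passing that shared context.
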(event EventBeginPlay
  (Utilities|FlowControl|Sequence
    (:then_0
      (bind _returnvalue (Game|SpawnActorfromClass "/Game/23_Interpreter/BP_TerminalExpression.BP_TerminalExpression_C" (Math|Transform|MakeTransform "0, 0, 0" "0, 0, 0" "1,1,1") "Undefined" 0 0))
      (Utilities|Array|Add (Variables|Default|GetExpressionList) _returnvalue))
    (:then_1
      (bind _returnvalue_2 (Game|SpawnActorfromClass "/Game/23_Interpreter/BP_TerminalExpression.BP_TerminalExpression_C" (Math|Transform|MakeTransform "0, 0, 0" "0, 0, 0" "1,1,1") "Undefined" 0 0))
      (Utilities|Array|Add (Variables|Default|GetExpressionList) _returnvalue_2))
    (:then_2
      (bind _returnvalue_3 (Game|SpawnActorfromClass "/Game/23_Interpreter/BP_NonTerminalExpression.BP_NonTerminalExpression_C" (Math|Transform|MakeTransform "0, 0, 0" "0, 0, 0" "1,1,1") "Undefined" 0 0))
      (Utilities|Array|Add (Variables|Default|GetExpressionList) _returnvalue_3))
    (:then_3
      (bind _returnvalue_4 (Game|SpawnActorfromClass "/Game/23_Interpreter/BP_InterpreterContext.BP_InterpreterContext_C" (Math|Transform|MakeTransform "0, 0, 0" "0, 0, 0" "1,1,1") "Undefined" 0 0))
      (for _array_element (Variables|Default|GetExpressionList)
        (Default|Interpret _array_element _returnvalue_4)))))

(fn ConstructionScript)